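; Interactable actor that shows an on-screen interaction prompt while the first-person character overlaps it.
; On BeginPlay it applies its configured mesh to the DefaultInteractable component.
; Begin and end overlap find top-level InteractableUI_BP widgets, set their text from the InteractableType enum, and show or hide them.
; It handles only the prompt and contains no interaction logic.
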(event EventBeginPlay
  ;[0 0 0] Sets up the interactable mesh
  (Components|StaticMesh|SetStaticMesh (Variables|Default|GetDefault_Interactable) (Variables|Default|GetInteractable_Mesh)))

(event Collision|EventActorEndOverlap
  (params (OtherActor :type Actor%20Object%20Reference))
  ;[0 0 0] Displays UI instructions for interaction
  (Utilities|Casting|CastToFirstPersonCharacter OtherActor)
  (bind _foundwidgets (Widget|GetAllWidgetsOfClass "/Game/Interactables/BlueprintsWidgets/InteractableUI_BP.InteractableUI_BP_C" true))
  (for _array_element _foundwidgets
    (Variables|/Game/Interactables/BlueprintsWidgets/InteractableUI_BP.InteractableUI_BP_C|SetInteractable_Type _array_element (Utilities|Text|ToText(String) (Utilities|String|EnumtoString (Variables|Default|GetInteractable_Type))))
    (Widget|SetVisibility _array_element "Hidden")))

(event Collision|EventActorBeginOverlap
  (params (OtherActor :type Actor%20Object%20Reference))
  ;[0 0 0] Displays UI instructions for interaction
  (Utilities|Casting|CastToFirstPersonCharacter OtherActor)
  (bind _foundwidgets (Widget|GetAllWidgetsOfClass "/Game/Interactables/BlueprintsWidgets/InteractableUI_BP.InteractableUI_BP_C" true))
  (for _array_element _foundwidgets
    (Variables|/Game/Interactables/BlueprintsWidgets/InteractableUI_BP.InteractableUI_BP_C|SetInteractable_Type _array_element (Utilities|Text|ToText(String) (Utilities|String|EnumtoString (Variables|Default|GetInteractable_Type))))
    (Widget|SetVisibility _array_element "Visible")))

(fn ConstructionScript)