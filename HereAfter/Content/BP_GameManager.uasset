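; Game manager that runs quest interactions: rope and well, mandragora plant, deer bones, casket, key door and torch.
; On Interact, it loops all Interactable_BP actors overlapping the player and branches on InteractableType.
; Progress booleans gate steps, with quest-name checks on water, plant and deer; the casket's BoxQuest check is unused.
; Steps show, hide or destroy props, complete quests through QuestMan, or rotate the door by timeline.
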(event EventBeginPlay
  (bind _outactors (Actor|GetAllActorsOfClass "BP_GameManager_C"))
  (Variables|Default|SetGameManager (Utilities|Array|Get(acopy) _outactors)))

(event Input|ActionEvents|InputActionInteract
  (params (Key :type Key%20Structure))
  ;[0 0 0] Prevent Doing Quests in the wrong order
  (:Pressed
    (bind _returnvalue (Class|QuestManager|GetCurrentQuest (Variables|Default|GetQuestMan)))
    (bind _returnvalue_2 (Class|Quest|GetName _returnvalue))
    (bind _returnvalue_3 (Class|QuestManager|GetCurrentQuest (Variables|Default|GetQuestMan)))
    (bind _returnvalue_4 (Class|Quest|GetName _returnvalue_3))
    (bind _returnvalue_5 (Class|QuestManager|GetCurrentQuest (Variables|Default|GetQuestMan)))
    (bind _returnvalue_6 (Class|Quest|GetName _returnvalue_5))
    (bind _returnvalue_7 (Class|QuestManager|GetCurrentQuest (Variables|Default|GetQuestMan)))
    (bind _returnvalue_8 (Class|Quest|GetName _returnvalue_7))
    (bind _outactors (Actor|GetAllActorsOfClass "/Game/Interactables/BlueprintsWidgets/Interactable_BP.Interactable_BP_C"))
    (for _array_element _outactors
      (if (Collision|IsOverlappingActor _array_element (Game|GetPlayerCharacter 0) :!class /Script/Engine.Actor)
        ;[0 0 0] Collecting Rope
        (if (Utilities|Enum|Equal(Enum) (Variables|/Game/Interactables/BlueprintsWidgets/Interactable_BP.Interactable_BP_C|GetInteractable_Type _array_element) "NewEnumerator0")
          (Development|PrintString "Picking up Rope")
          (Variables|Default|SetCollectRope true)
          (Actor|DestroyActor _array_element)
          (else
            ;[0 0 0] Attaching Rope
            (if (and (Utilities|Enum|Equal(Enum) (Variables|/Game/Interactables/BlueprintsWidgets/Interactable_BP.Interactable_BP_C|GetInteractable_Type _array_element) "NewEnumerator2") (Utilities|Enum|Equal(Enum) _returnvalue_2 "WaterQuest"))
              (Development|PrintString "Attaching Rope")
              (if (Variables|Default|GetCollectRope)
                (Variables|Default|SetAttachRope true)
                (Variables|Default|SetCollectRope false)
                (Variables|Default|SetAquiredWater true)
                (bind _returnvalue_9 (Class|QuestManager|GetCurrentQuest (Variables|/Script/HereAfter.MyGameManager|GetQuestMan (Variables|Default|GetGameManager))))
                (Class|Quest|SetCompleted _returnvalue_9 true)
                (bind _ropetowell (Variables|Default|GetRopeToWell)
                  (:then
                    (Rendering|SetVisibility (Variables|/Script/Engine.Actor|GetRootComponent _ropetowell) true false)
                    (Development|PrintString "IT WORK"))
                  (:else
                    (Development|PrintString "Hello" true true "(R=0.000000,G=0.660000,B=1.000000,A=1.000000)" 5.0))))
              (else
                ;[0 0 0] Mandragora
                (if (and (Utilities|Enum|Equal(Enum) (Variables|/Game/Interactables/BlueprintsWidgets/Interactable_BP.Interactable_BP_C|GetInteractable_Type _array_element) "NewEnumerator8") (Utilities|Enum|Equal(Enum) _returnvalue_4 "PlantQuest"))
                  (Development|PrintString "Get Dead PLant ")
                  (Variables|Default|SetHasDeadPlant true)
                  (Actor|DestroyActor _array_element)
                  (elif (and (Utilities|Enum|Equal(Enum) (Variables|/Game/Interactables/BlueprintsWidgets/Interactable_BP.Interactable_BP_C|GetInteractable_Type _array_element) "NewEnumerator9") (Variables|Default|GetHasDeadPlant))
                    (Development|PrintString "Plant it")
                    (bind _mandragora_planting (Variables|Default|GetMandragora-Planting)
                      (:then
                        (Rendering|SetVisibility (Variables|/Script/Engine.Actor|GetRootComponent _mandragora_planting) true false)
                        (Variables|Default|SetPlanted true))
                      (:else
                        (Development|PrintString "fdklh kldg hldsfjgldflgldkfgjldfgjdlfgldfjgldkjg" true true "(R=1.000000,G=0.000000,B=0.000000,A=1.000000)")))
                    (elif (and (Utilities|Enum|Equal(Enum) (Variables|/Game/Interactables/BlueprintsWidgets/Interactable_BP.Interactable_BP_C|GetInteractable_Type _array_element) "NewEnumerator10") (Variables|Default|GetPlanted))
                      (Development|PrintString "Dug the plant")
                      (bind _mandragora_planting_2 (Variables|Default|GetMandragora-Planting)
                        (:then
                          (Rendering|SetVisibility (Variables|/Script/Engine.Actor|GetRootComponent _mandragora_planting_2) false false)
                          (Variables|Default|SetAdquiredPlant true)
                          (bind _returnvalue_10 (Class|QuestManager|GetCurrentQuest (Variables|/Script/HereAfter.MyGameManager|GetQuestMan (Variables|Default|GetGameManager))))
                          (Class|Quest|SetCompleted _returnvalue_10 true))
                        (:else
                          (Development|PrintString "IT DOESNT WORK FFS")))
                      (else
                        ;[0 0 0] Kill Deer
                        (if (and (Utilities|Enum|Equal(Enum) (Variables|/Game/Interactables/BlueprintsWidgets/Interactable_BP.Interactable_BP_C|GetInteractable_Type _array_element) "NewEnumerator4") (Utilities|Enum|Equal(Enum) _returnvalue_6 "DeerQuest"))
                          (Development|PrintString "Kill Deer")
                          (Variables|/Game/Interactables/BP_Deer.BP_Deer_C|SetDeathOfDeer (Variables|Default|GetDeer) true)
                          (bind _deerbones (Variables|Default|GetDeerBones)
                            (:then
                              (Rendering|SetVisibility (Variables|/Script/Engine.Actor|GetRootComponent _deerbones) true false))
                            (:else
                              (Development|PrintString "KILL ME NOW" true true "(R=1.000000,G=0.000000,B=0.000000,A=1.000000)")))
                          (elif (and (Utilities|Enum|Equal(Enum) (Variables|/Game/Interactables/BlueprintsWidgets/Interactable_BP.Interactable_BP_C|GetInteractable_Type _array_element) "NewEnumerator11") (Variables|/Game/Interactables/BP_Deer.BP_Deer_C|GetDeathOfDeer (Variables|Default|GetDeer)))
                            (Variables|Default|SetAdquiredBone true)
                            (bind _gamemanager (Variables|Default|GetGameManager)
                              (:then
                                (bind _returnvalue_11 (Class|QuestManager|GetCurrentQuest (Variables|/Script/HereAfter.MyGameManager|GetQuestMan _gamemanager)))
                                (Class|Quest|SetCompleted _returnvalue_11 true)
                                (Actor|DestroyActor (Variables|Default|GetDeerBones)))
                              (:else
                                (Development|PrintString "MY ASSHOLE IS BURNING LOL" true true "(R=1.000000,G=0.000000,B=0.000000,A=1.000000)")))
                            (else
                              ;[0 0 0] Open Casket
                              (if (Utilities|Enum|Equal(Enum) (Variables|/Game/Interactables/BlueprintsWidgets/Interactable_BP.Interactable_BP_C|GetInteractable_Type _array_element) "NewEnumerator12")
                                (Variables|Default|SetHasSpade true)
                                (Actor|DestroyActor (Variables|Default|GetSpade))
                                (elif (and (Utilities|Enum|Equal(Enum) (Variables|/Game/Interactables/BlueprintsWidgets/Interactable_BP.Interactable_BP_C|GetInteractable_Type _array_element) "NewEnumerator13") (Variables|Default|GetHasSpade))
                                  (Variables|Default|SetDugDirt true)
                                  (Actor|DestroyActor (Variables|Default|GetDirt))
                                  (elif (and (Utilities|Enum|Equal(Enum) (Variables|/Game/Interactables/BlueprintsWidgets/Interactable_BP.Interactable_BP_C|GetInteractable_Type _array_element) "NewEnumerator5") (Variables|Default|GetDugDirt))
                                    (Development|PrintString "Open Casket")
                                    (Variables|Default|SetAdquiredBox true)
                                    (bind _returnvalue_12 (Class|QuestManager|GetCurrentQuest (Variables|/Script/HereAfter.MyGameManager|GetQuestMan (Variables|Default|GetGameManager))))
                                    (Class|Quest|SetCompleted _returnvalue_12 true)
                                    (Variables|Default|SetAdquiredKey true)
                                    (Actor|DestroyActor (Variables|Default|GetCasket))
                                    (else
                                      ;[0 0 0] Door Open
                                      (if (and (Utilities|Enum|Equal(Enum) (Variables|/Game/Interactables/BlueprintsWidgets/Interactable_BP.Interactable_BP_C|GetInteractable_Type _array_element) "NewEnumerator6") (Variables|Default|GetAdquiredKey))
                                        (Development|PrintString "Has Key")
                                        (bind _rotateangle (Timeline|Timeline_0 Play)
                                          (:Update
                                            (Transformation|SetActorRotation _array_element (Math|Rotator|MakeRotator 0.0 0.0 _rotateangle))))
                                        (else
                                          ;[0 0 0] Getting Torch
                                          (if (Utilities|Enum|Equal(Enum) (Variables|/Game/Interactables/BlueprintsWidgets/Interactable_BP.Interactable_BP_C|GetInteractable_Type _array_element) "NewEnumerator7")
                                            (Development|PrintString "Getting Torch")
                                            (bind _asfirst_person_character (Utilities|Casting|CastToFirstPersonCharacter (Game|GetPlayerCharacter 0)))
                                            (Rendering|SetVisibility (Variables|/Game/FirstPersonCPP/Blueprints/FirstPersonCharacter.FirstPersonCharacter_C|GetTemp%20Torch _asfirst_person_character) true false)
                                            (Rendering|SetVisibility (Variables|/Game/FirstPersonCPP/Blueprints/FirstPersonCharacter.FirstPersonCharacter_C|GetP_TorchFire _asfirst_person_character) true false)
                                            (Variables|Default|SetHoldingTorch true)))))))))))))))))))))))

(fn ConstructionScript)